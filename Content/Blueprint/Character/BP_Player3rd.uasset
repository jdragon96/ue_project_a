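; BP_Player3rd is a player Blueprint, apparently third-person, that keeps a Weapon component orbiting around the actor.
; Each Tick advances Angle by RotationSpeed without delta-time scaling, so orbit speed depends on frame rate.
; Cos and Sin of Angle place the Weapon on a fixed-radius horizontal circle around the actor, setting its world transform with zero rotation and no sweep.
; BeginPlay, overlap and construction logic are empty.
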(event `self.ReceiveBeginPlay`)

(event `self.ReceiveTick`
  (params (DeltaSeconds :type "Float (single-precision)"))
  (bind _output_get (set `self.Angle` (+ (`self.Angle`) (`self.RotationSpeed`))))
  (`SceneComponent.K2_SetWorldTransform` (`self.Weapon`) (`KismetMathLibrary.MakeTransform` (+ (`self.K2_GetActorLocation`) (`KismetMathLibrary.MakeVector` (* (`KismetMathLibrary.Cos` _output_get) 1000.0) (* (`KismetMathLibrary.Sin` _output_get) 1000.0)))) false false))

(fn `UserConstructionScript`)